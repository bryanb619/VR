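; Cart actor that rides along the spline of a referenced spline actor, starting automatically on BeginPlay.
; The Move event sets the MovingCart timeline's play rate to the inverse of CartSpeed, so a larger CartSpeed slows the timeline.
; Each update maps the timeline's Blend value to a distance along the spline and applies that world location and rotation to the cart.
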(event `self.ReceiveBeginPlay`
  (`self.Move`))

(event `Move`
  (bind _spline (`/Game/Blueprints/Cart/Spline_BP.Spline` (`self.spline_reference`)))
  (bind _returnvalue (`KismetMathLibrary.Lerp` 0.0 (`SplineComponent.GetSplineLength` (`/Game/Blueprints/Cart/Spline_BP.Spline` (`self.spline_reference`))) (`self.Blend`)))
  (`TimelineComponent.SetPlayRate` (`self.MovingCart`) (/ 1.0 (`self.CartSpeed`)))
  (bind (_direction _blend) (`Timeline|MovingCart`)
    (:`Update`
      (set `self.Blend` _blend)
      (`self.K2_SetActorLocationAndRotation` (`SplineComponent.GetLocationAtDistanceAlongSpline` _spline _returnvalue "World") (`SplineComponent.GetRotationAtDistanceAlongSpline` _spline _returnvalue "World")))))

(fn `UserConstructionScript`)