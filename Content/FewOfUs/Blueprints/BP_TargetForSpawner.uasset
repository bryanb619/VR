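; BP_TargetForSpawner is a spawn point that cycles an actor of the ItemsToSpawn class at its own location and rotation.
; On BeginPlay, AttemptToSpawn spawns and stores the actor unless CurrentItem is still valid, in which case it prints a message.
; The spawned actor is attached to the spawner, destroyed after a fixed seven-second delay, then respawned in a continuous loop.
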(event `self.ReceiveBeginPlay`
  (`self.AttemptToSpawn` :!label _label)
  (if (`self.bSpawnItem`)
    (`self.K2_AttachToActor` (`self.currentItem`) self "None" "KeepWorld" "KeepWorld" "KeepWorld" true)
    (`KismetSystemLibrary.Delay` 7.0)
    (`self.K2_DestroyActor` (`self.currentItem`))
    (goto _label)))

(fn `AttemptToSpawn`
  (`/Engine/EditorBlueprintResources/StandardMacros.IsValid` (`self.currentItem`)
    (:`Is Valid`
      (`KismetSystemLibrary.PrintString` "Item Already Spawned"))
    (:`Is Not Valid`
      (set `self.bSpawnItem` true)
      (`self.SpawnItem`))))

(fn `SpawnItem`
  (bind _returnvalue (`|SpawnActorFromClass` (`self.ItemsToSpawn`) (`KismetMathLibrary.MakeTransform` (`self.K2_GetActorLocation`) (`self.K2_GetActorRotation`)) "AlwaysSpawn" "OverrideRootScale" self null))
  (set `self.currentItem` _returnvalue))

(fn `UserConstructionScript`)